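; Player character that directs an AIP_Pawn in the level through mouse clicks and a state-change input.
; On BeginPlay it shows the cursor, adds the Enhanced Input mapping context and caches the first AIP_Pawn found.
; A click traces under the cursor, spawns a BP_MyActorToTarget there at a fixed height, assigns it as the pawn's Target and prints the location.
; The change-state input calls ChangeState on that pawn.
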(event Input|EnhancedActionEvents|EnhancedInputActionIA_Click
  (params (ActionValue :type Boolean) (ElapsedSeconds :type Float%20%28double-precision%29) (TriggeredSeconds :type Float%20%28double-precision%29) (InputAction :type Input%20Action%20Object%20Reference :default "/Game/Inputs/IA_Click.IA_Click"))
  (bind _returnvalue (Game|GetPlayerController 0))
  (bind _hitresult (Game|Player|GetHitResultUnderCursorbyChannel _returnvalue "TraceTypeQuery2" true))
  (:Completed
    (bind _returnvalue_2 (Game|SpawnActorfromClass "/Game/BP_MyActorToTarget.BP_MyActorToTarget_C" (Math|Transform|MakeTransform (Math|Vector|MakeVector (.x (.location _hitresult)) (.y (.location _hitresult)) 1e+01) "0, 0, 0" "1.000000,1.000000,1.000000") "Undefined" "MultiplyWithRoot" 0 0))
    (Variables|/Script/ProjectMPIA1.AIPawn|SetTarget (Variables|Default|GetPawn) _returnvalue_2)
    (Development|PrintString (Utilities|String|ToString(Vector2d) (Math|Vector2D|MakeVector2D (.x (.location _hitresult)) (.y (.location _hitresult)))))))

(event Input|EnhancedActionEvents|EnhancedInputActionIA_ChangeState
  (params (ActionValue :type Boolean) (ElapsedSeconds :type Float%20%28double-precision%29) (TriggeredSeconds :type Float%20%28double-precision%29) (InputAction :type Input%20Action%20Object%20Reference :default "/Game/Inputs/IA_ChangeState.IA_ChangeState"))
  (:Completed
    (Default|ChangeState (Variables|Default|GetPawn))))

(event EventBeginPlay
  (Variables|/Script/Engine.PlayerController|SetbShowMouseCursor (Game|GetPlayerController (Game|GetPlayerState 0)) true)
  (Input|AddMappingContext (PlayerController|LocalPlayerSubsystems|GetEnhancedInputLocalPlayerSubsystem (Game|GetPlayerController 0)) "/Game/Inputs/IMC_Default.IMC_Default" 0 "(bIgnoreAllPressedKeysUntilRelease=True,bForceImmediately=False,bNotifyUserSettings=False)")
  (bind _outactors (Actor|GetAllActorsOfClass "/Game/AIP_Pawn.AIP_Pawn_C"))
  (Variables|Default|SetPawn (Utilities|Array|Get(acopy) _outactors)))

(fn ConstructionScript)